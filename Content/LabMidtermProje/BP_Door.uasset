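; BP_Door is an interactable door that opens when the game mode's key count exactly equals the door's key number.
; On BeginPlay it caches GM_MainGM, and Interact plays the Door_Rotate timeline to lerp the cube's relative location between start and finish points.
; Despite the timeline's name, the door slides rather than rotates.
; The construction script applies a configurable material to the cube.
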(event EventBeginPlay
  (bind _asgm_main_gm (Utilities|Casting|CastToGM_MainGM (Game|GetGameMode)))
  (Variables|Default|SetAs%20GM%20Main%20GM _asgm_main_gm))

(event EventInteract
  (if (== (Variables|/Game/LabMidtermProje/GM_MainGM.GM_MainGM_C|GetKeys (Variables|Default|GetAs%20GM%20Main%20GM)) (Variables|Default|GetKeyNumber))
    (bind _newtrack_0 (Timeline|Door_Rotate Play)
      (:Update
        (Transformation|SetRelativeLocation (Variables|Default|GetCube) (Math|Vector|Lerp(Vector) (Variables|Default|GetStartLoc) (Variables|Default|GetFinishLoc) _newtrack_0) false false)))))

(fn ConstructionScript
  (Rendering|Material|SetMaterial (Variables|Default|GetCube) 0 (Variables|Default|GetMaterial)))