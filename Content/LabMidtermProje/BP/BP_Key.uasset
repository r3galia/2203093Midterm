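; BP_Key is a collectible key actor that records its key number in the game mode when interacted with.
; On BeginPlay it caches a reference to GM_MainGM.
; Interact overwrites the game mode's Keys value with its KeyNumber, prints a collection message, then destroys the actor.
; The Construction Script applies the Material variable to the Key component, so each instance can have its own look.
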(event EventBeginPlay
  (bind _asgm_main_gm (Utilities|Casting|CastToGM_MainGM (Game|GetGameMode)))
  (Variables|Default|SetAs%20GM%20Main%20GM _asgm_main_gm))

(event EventInteract
  (bind _output_get (Variables|/Game/LabMidtermProje/GM_MainGM.GM_MainGM_C|SetKeys (Variables|Default|GetAs%20GM%20Main%20GM) (Variables|Default|GetKeyNumber)))
  (Development|PrintString (Utilities|String|Append "Key" (Utilities|String|ToString(Integer) _output_get) "Collected"))
  (Actor|DestroyActor))

(fn ConstructionScript
  (Rendering|Material|SetMaterial (Variables|Default|GetKey) 0 (Variables|Default|GetMaterial)))