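; BP_AxeTrap is a swinging axe trap that triggers when the third-person player character enters its box.
; A timeline rolls the axe 180 degrees from its starting rotation, then a short delay snaps it back and rearms the trap.
; The axe's own collider applies fixed damage to the character on overlap.
; Both the trigger and the damage are skipped while the player's IsDeactivatedTrap3 flag is set.
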(event OnComponentBeginOverlap(Box)
  (params (OverlappedComponent :type Primitive%20Component%20Object%20Reference) (OtherActor :type Actor%20Object%20Reference) (OtherComp :type Primitive%20Component%20Object%20Reference) (OtherBodyIndex :type Integer) (bFromSweep :type Boolean) (SweepResult :type Hit%20Result%20Structure%20%28by%20ref%29))
  (bind _currot (Variables|Default|GetCurRot))
  (bind (_roll _pitch _yaw) (Math|Rotator|BreakRotator _currot))
  (if (not (Variables|/Game/LabMidtermProje/BP/BP_ThirdPersonCharacter.BP_ThirdPersonCharacter_C|GetisDeactivatedTrap3 (Variables|Default|GetAs%20BP%20Third%20Person%20Character)))
    (Utilities|Casting|CastToBP_ThirdPersonCharacter OtherActor)
    (if (not (Variables|Default|GetisActivated))
      (Variables|Default|SetisActivated true)
      (Utilities|FlowControl|Sequence
        (:then_0
          (bind _swingfloat (Timeline|AxeSwing PlayFromStart)
            (:Update
              (Transformation|SetRelativeRotation (Variables|Default|GetAxe) (Math|Rotator|Lerp(Rotator) (Variables|Default|GetCurRot) (Math|Rotator|MakeRotator (+ _roll -1.8e+02) _pitch _yaw) _swingfloat) false false))))
        (:then_1
          (Utilities|FlowControl|Delay 3.0)
          (Transformation|SetRelativeRotation (Variables|Default|GetAxe) (Variables|Default|GetCurRot) false false)
          (Variables|Default|SetisActivated false))))))

(event OnComponentBeginOverlap(AxeColl)
  (params (OverlappedComponent :type Primitive%20Component%20Object%20Reference) (OtherActor :type Actor%20Object%20Reference) (OtherComp :type Primitive%20Component%20Object%20Reference) (OtherBodyIndex :type Integer) (bFromSweep :type Boolean) (SweepResult :type Hit%20Result%20Structure%20%28by%20ref%29))
  (if (not (Variables|/Game/LabMidtermProje/BP/BP_ThirdPersonCharacter.BP_ThirdPersonCharacter_C|GetisDeactivatedTrap3 (Variables|Default|GetAs%20BP%20Third%20Person%20Character)))
    (bind _asbp_third_person_character (Utilities|Casting|CastToBP_ThirdPersonCharacter OtherActor))
    (Game|Damage|ApplyDamage _asbp_third_person_character 2e+01 0 0)))

(event EventBeginPlay
  (Variables|Default|SetCurRot (Variables|/Script/Engine.SceneComponent|GetRelativeRotation (Variables|Default|GetAxe)))
  (bind _asbp_third_person_character (Utilities|Casting|CastToBP_ThirdPersonCharacter (Game|GetPlayerCharacter 0)))
  (Variables|Default|SetAs%20BP%20Third%20Person%20Character _asbp_third_person_character))

(fn ConstructionScript)