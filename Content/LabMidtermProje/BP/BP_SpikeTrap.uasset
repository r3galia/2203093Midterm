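; Spike trap actor that thrusts spikes along its local X axis and damages the player character, unless that character's IsDeactivatedTrap1 flag is set.
; One box overlap plays a timeline that lerps the spikes from their starting relative location.
; A second box overlap applies TrapDamage independently.
; Each trigger has its own DoOnce gate, re-armed by a delay to act as a cooldown.
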(event OnComponentBeginOverlap(Box)
  (params (OverlappedComponent :type Primitive%20Component%20Object%20Reference) (OtherActor :type Actor%20Object%20Reference) (OtherComp :type Primitive%20Component%20Object%20Reference) (OtherBodyIndex :type Integer) (bFromSweep :type Boolean) (SweepResult :type Hit%20Result%20Structure%20%28by%20ref%29))
  (bind _startvector (Variables|Default|GetStartVector))
  (bind (_x _y _z) (Math|Vector|BreakVector _startvector))
  (if (not (Variables|/Game/LabMidtermProje/BP/BP_ThirdPersonCharacter.BP_ThirdPersonCharacter_C|GetisDeactivatedTrap1 (Variables|Default|GetAs%20BP%20Third%20Person%20Character)))
    (Utilities|Casting|CastToBP_ThirdPersonCharacter OtherActor)
    (Utilities|FlowControl|DoOnce false
      (:Completed
        (bind _spikeattack (Timeline|Spike PlayFromStart)
          (:Update
            (Transformation|SetRelativeLocation (Variables|Default|GetSpikes) (Math|Vector|Lerp(Vector) (Variables|Default|GetStartVector) (Math|Vector|MakeVector (+ _x -4.5e+02) _y _z) _spikeattack) false false)
            (Utilities|FlowControl|Delay 4.0)
            (CallFunction|ResetTrap)))))))

(event OnComponentBeginOverlap(Box1)
  (params (OverlappedComponent :type Primitive%20Component%20Object%20Reference) (OtherActor :type Actor%20Object%20Reference) (OtherComp :type Primitive%20Component%20Object%20Reference) (OtherBodyIndex :type Integer) (bFromSweep :type Boolean) (SweepResult :type Hit%20Result%20Structure%20%28by%20ref%29))
  (if (not (Variables|/Game/LabMidtermProje/BP/BP_ThirdPersonCharacter.BP_ThirdPersonCharacter_C|GetisDeactivatedTrap1 (Variables|Default|GetAs%20BP%20Third%20Person%20Character)))
    (bind _asbp_third_person_character (Utilities|Casting|CastToBP_ThirdPersonCharacter OtherActor))
    (Utilities|FlowControl|DoOnce false :!label _label
      (:Completed
        (Game|Damage|ApplyDamage _asbp_third_person_character (Variables|Default|GetTrapDamage) 0 0)
        (Utilities|FlowControl|Delay 4.0)
        (goto _label Reset)))))

(event Custom|ResetTrap
  (bind _startvector (Variables|Default|GetStartVector))
  (bind (_x _y _z) (Math|Vector|BreakVector _startvector))
  (Utilities|FlowControl|DoOnce false) ; enters at Reset
)

(event EventBeginPlay
  (Variables|Default|SetStartVector (Variables|/Script/Engine.SceneComponent|GetRelativeLocation (Variables|Default|GetSpikes)))
  (bind _asbp_third_person_character (Utilities|Casting|CastToBP_ThirdPersonCharacter (Game|GetPlayerCharacter 0)))
  (Variables|Default|SetAs%20BP%20Third%20Person%20Character _asbp_third_person_character))

(event Collision|EventActorBeginOverlap
  (params (OtherActor :type Actor%20Object%20Reference)))

(event EventTick
  (params (DeltaSeconds :type Float%20%28single-precision%29)))

(fn ConstructionScript)