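; Gas trap actor that deals steady damage over time to the player character inside its DamageArea.
; Entering the area starts a looping timer that calls GasDamage to damage player 0, and leaving clears it.
; Both overlap handlers act only while the cached player's IsDeactivatedTrap2 flag is false, so deactivating the trap mid-overlap leaves the timer running on exit.
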(event OnComponentBeginOverlap(DamageArea)
  (params (OverlappedComponent :type Primitive%20Component%20Object%20Reference) (OtherActor :type Actor%20Object%20Reference) (OtherComp :type Primitive%20Component%20Object%20Reference) (OtherBodyIndex :type Integer) (bFromSweep :type Boolean) (SweepResult :type Hit%20Result%20Structure%20%28by%20ref%29))
  (if (not (Variables|/Game/LabMidtermProje/BP/BP_ThirdPersonCharacter.BP_ThirdPersonCharacter_C|GetisDeactivatedTrap2 (Variables|Default|GetAs%20BP%20Third%20Person%20Character)))
    (Utilities|Casting|CastToBP_ThirdPersonCharacter OtherActor)
    (Utilities|Time|SetTimerbyFunctionName 0 "GasDamage" 0.2 true)))

(event OnComponentEndOverlap(DamageArea)
  (params (OverlappedComponent :type Primitive%20Component%20Object%20Reference) (OtherActor :type Actor%20Object%20Reference) (OtherComp :type Primitive%20Component%20Object%20Reference) (OtherBodyIndex :type Integer))
  (if (not (Variables|/Game/LabMidtermProje/BP/BP_ThirdPersonCharacter.BP_ThirdPersonCharacter_C|GetisDeactivatedTrap2 (Variables|Default|GetAs%20BP%20Third%20Person%20Character)))
    (Utilities|Casting|CastToBP_ThirdPersonCharacter OtherActor)
    (Utilities|Time|ClearTimerbyFunctionName 0 "GasDamage")))

(event Custom|GasDamage
  (bind _asbp_third_person_character (Utilities|Casting|CastToBP_ThirdPersonCharacter (Game|GetPlayerCharacter 0)))
  (Game|Damage|ApplyDamage _asbp_third_person_character 1.0 0 0))

(event EventBeginPlay
  (bind _asbp_third_person_character (Utilities|Casting|CastToBP_ThirdPersonCharacter (Game|GetPlayerCharacter 0)))
  (Variables|Default|SetAs%20BP%20Third%20Person%20Character _asbp_third_person_character))

(fn ConstructionScript)