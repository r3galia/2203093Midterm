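; BP_TrapDeactivate is an interactable actor that disables one of three traps.
; It caches the player's BP_ThirdPersonCharacter on BeginPlay.
; On Interact, DeactivateType selects which trap-deactivated flag to set on that character, prints a confirmation and destroys the actor.
; The construction script applies a configurable material to its static mesh.
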(event EventBeginPlay
  (bind _asbp_third_person_character (Utilities|Casting|CastToBP_ThirdPersonCharacter (Game|GetPlayerCharacter 0)))
  (Variables|Default|SetAs%20BP%20Third%20Person%20Character _asbp_third_person_character))

(event EventInteract
  (switch int (Variables|Default|GetDeactivateType)
    (:0
      (Variables|/Game/LabMidtermProje/BP/BP_ThirdPersonCharacter.BP_ThirdPersonCharacter_C|SetisDeactivatedTrap1 (Variables|Default|GetAs%20BP%20Third%20Person%20Character) true)
      (Development|PrintString "TRAP 1 Deactivated"))
    (:1
      (Variables|/Game/LabMidtermProje/BP/BP_ThirdPersonCharacter.BP_ThirdPersonCharacter_C|SetisDeactivatedTrap2 (Variables|Default|GetAs%20BP%20Third%20Person%20Character) true)
      (Development|PrintString "TRAP 2 Deactivated"))
    (:2
      (Variables|/Game/LabMidtermProje/BP/BP_ThirdPersonCharacter.BP_ThirdPersonCharacter_C|SetisDeactivatedTrap3 (Variables|Default|GetAs%20BP%20Third%20Person%20Character) true)
      (Development|PrintString "TRAP 3 Deactivated")))
  (Actor|DestroyActor))

(fn ConstructionScript
  (Rendering|Material|SetMaterial (Variables|Default|GetStaticMesh) 0 (Variables|Default|GetMaterial)))