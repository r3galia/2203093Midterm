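; BP_Gold is an interactable gold pickup that adds a random amount of gold to the player's total in GM_MainGM.
; On BeginPlay it caches the game mode, rolls the gold amount, and hides extra Gold components so the visible pile reflects one of three value tiers.
; Interact runs once through a DoOnce, adds the amount to CurrentGold, prints the new total and destroys the actor.
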(event EventInteract
  (bind _as_gm_main_gm (Variables|Default|GetAs%20GM%20Main%20GM))
  (Utilities|FlowControl|DoOnce false
    (:Completed
      (bind _output_get (Variables|/Game/LabMidtermProje/GM_MainGM.GM_MainGM_C|SetCurrentGold _as_gm_main_gm (+ (Variables|/Game/LabMidtermProje/GM_MainGM.GM_MainGM_C|GetCurrentGold _as_gm_main_gm) (Variables|Default|GetgoldCount))))
      (Development|PrintString (Utilities|String|ToString(Integer) _output_get))
      (Actor|DestroyActor))))

(event EventBeginPlay
  (bind _asgm_main_gm (Utilities|Casting|CastToGM_MainGM (Game|GetGameMode)))
  (Variables|Default|SetAs%20GM%20Main%20GM _asgm_main_gm)
  (Variables|Default|SetgoldCount (Math|Random|RandomIntegerinRange 1 99))
  (if (<= (Variables|Default|GetgoldCount) 25)
    (Rendering|SetVisibility (Variables|Default|GetGold3) false false)
    (Rendering|SetVisibility (Variables|Default|GetGold2) false false)
    (elif (<= (Variables|Default|GetgoldCount) 75)
      (Rendering|SetVisibility (Variables|Default|GetGold3) false false))))

(fn ConstructionScript)